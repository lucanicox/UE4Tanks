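; BP_PawnTurret is an enemy turret Blueprint that handles its own destruction and can drop a pickup.
; On HandleDestruction it makes a random boolean roll, calls SpawnPickup on success, then destroys itself.
; SpawnPickup spawns a random class from PickupsArray at a small random positive X/Y offset from the turret, at the same height, ignoring collision.
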(event EventBeginPlay)

(event Collision|EventActorBeginOverlap
  (params (OtherActor :type Actor%20Object%20Reference)))

(event EventTick
  (params (DeltaSeconds :type Float%20%28single-precision%29)))

(event EventHandleDestruction
  (if (Math|Random|RandomBool)
    (CallFunction|SpawnPickup))
  (Actor|DestroyActor))

(fn ConstructionScript)

(fn SpawnPickup
  (bind _returnvalue (Transformation|GetActorLocation))
  (Game|SpawnActorfromClass (.OutItem (Utilities|Array|Random (Variables|Default|GetPickupsArray))) (Math|Transform|MakeTransform (Math|Vector|MakeVector (+ (Math|Random|RandomFloatinRange 5e+01 1e+02) (.x _returnvalue)) (+ (Math|Random|RandomFloatinRange 5e+01 1e+02) (.y _returnvalue)) (.z _returnvalue)) "0, 0, 0" "1,1,1") "AlwaysSpawn" 0 0))