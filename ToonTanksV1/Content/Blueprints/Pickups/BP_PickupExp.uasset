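; BP_PickupExp is an experience pickup that grants XP to the player and can trigger a level-up.
; On PickedUp it adds ExpGained to the Experience stored in BP_GMLevelUp, prints the total, and asks that game mode whether it causes a level-up.
; A level-up pauses the game, shows the mouse cursor and opens WBP_LevelUp.
; The pickup then destroys itself.
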(event EventBeginPlay)

(event Collision|EventActorBeginOverlap
  (params (OtherActor :type Actor%20Object%20Reference)))

(event EventTick
  (params (DeltaSeconds :type Float%20%28single-precision%29)))

(event EventPickedUp
  (bind _returnvalue (Game|GetPlayerController 0))
  (bind _asbp_gmlevel_up (Utilities|Casting|CastToBP_GMLevelUp (Game|GetGameMode)))
  (bind _output_get (Variables|/Script/ToonTanksV1.LevelUpGameMode|SetExperience _asbp_gmlevel_up (+ (Variables|/Script/ToonTanksV1.LevelUpGameMode|GetExperience _asbp_gmlevel_up) (Variables|Default|GetExpGained))))
  (Development|PrintString (Utilities|String|ToString(Integer) _output_get))
  (bind _returnvalue_2 (Class|LevelUpGameMode|LevelUp _asbp_gmlevel_up _output_get))
  (if _returnvalue_2
    (Game|SetGamePaused true)
    (Variables|/Script/Engine.PlayerController|SetbShowMouseCursor _returnvalue true)
    (bind _returnvalue_3 (UserInterface|CreateWidget "/Game/Blueprints/HUD/WBP_LevelUp.WBP_LevelUp_C" _returnvalue))
    (UserInterface|Viewport|AddtoViewport _returnvalue_3 0))
  (Actor|DestroyActor))

(fn ConstructionScript)