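; BP_GMLevelUp, apparently a game mode, handles the start and end screens of a match.
; StartGame shows the WBP_StartGameHUD widget for about three seconds, then removes it.
; GameOver shows WBP_EndGame with win or loss text from its WonGame flag, then opens MainMenu after a short delay.
; BeginPlay and Tick are unused, and nothing in this file calls either event.
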(event EventBeginPlay)

(event EventTick
  (params (DeltaSeconds :type Float%20%28single-precision%29)))

(event EventStartGame
  (bind _returnvalue (UserInterface|CreateWidget "/Game/Blueprints/HUD/WBP_StartGameHUD.WBP_StartGameHUD_C"))
  (UserInterface|Viewport|AddtoViewport _returnvalue 0)
  (Utilities|FlowControl|Delay 3.1)
  (Widget|RemovefromParent _returnvalue))

(event EventGameOver
  (params (bWonGame :type Boolean))
  (bind _returnvalue (UserInterface|CreateWidget "/Game/Blueprints/HUD/WBP_EndGame.WBP_EndGame_C"))
  (UserInterface|Viewport|AddtoViewport _returnvalue 0)
  (Rendering|Components|TextRender|SetText (Variables|/Game/Blueprints/HUD/WBP_EndGame.WBP_EndGame_C|GetGameOverText _returnvalue) (select bWonGame "YOU WON!" "YOU LOST!"))
  (Utilities|FlowControl|Delay 2.5)
  (Game|OpenLevel(byName) "MainMenu"))

(fn ConstructionScript)